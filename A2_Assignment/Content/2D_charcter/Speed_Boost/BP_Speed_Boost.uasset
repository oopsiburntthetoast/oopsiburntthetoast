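; BP_Speed_Boost is a single-use pickup that gives BP_Player a brief speed boost.
; On capsule overlap it attaches a Niagara effect to the player's mesh, hides its own effect, destroys the capsule and plays activation and wind sounds.
; It raises the player's max walk speed, then lowers it to a hardcoded value after a short delay.
; It also changes its own CustomTimeDilation at both steps.
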(event OnComponentBeginOverlap(Capsule)
  (params (OverlappedComponent :type Primitive%20Component%20Object%20Reference) (OtherActor :type Actor%20Object%20Reference) (OtherComp :type Primitive%20Component%20Object%20Reference) (OtherBodyIndex :type Integer) (bFromSweep :type Boolean) (SweepResult :type Hit%20Result%20Structure%20%28by%20ref%29))
  ;[0.15 0.15 0.15 0.5] speed boost
  (bind _asbp_player (Utilities|Casting|CastToBP_Player OtherActor))
  (Niagara|SpawnSystemAttached "/Game/2D_charcter/Speed_Boost/Basic_VFX/Niagara/NS_Basic_14.NS_Basic_14" (Variables|/Script/Engine.Character|GetMesh _asbp_player) "None" "0, 0, 0" "0, 0, 0" "KeepRelativeOffset" false)
  (Rendering|SetVisibility (Variables|Default|GetNiagara) false false)
  (Components|DestroyComponent (Variables|Default|GetCapsule))
  (Audio|PlaySound2D "/Game/2D_charcter/Speed_Boost/SW_ActivateSpeed.SW_ActivateSpeed" 1.0 1.0 0.0 0 0)
  (Variables|/Script/Engine.CharacterMovementComponent|SetMaxWalkSpeed (Variables|/Script/Engine.Character|GetCharacterMovement _asbp_player) 1.2e+03)
  (Variables|Default|SetCustomTimeDilation 1.0)
  (Audio|PlaySound2D "/Game/2D_charcter/Speed_Boost/SW_BoostWind.SW_BoostWind" 1.0 1.0 0.0 0 0)
  (Utilities|FlowControl|Delay 1.0)
  (Variables|/Script/Engine.CharacterMovementComponent|SetMaxWalkSpeed (Variables|/Script/Engine.Character|GetCharacterMovement _asbp_player) 6e+02)
  (Variables|Default|SetCustomTimeDilation 0.5))

(fn ConstructionScript)